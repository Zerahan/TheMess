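; GenericFunctions is a pair of helper functions that convert between 2D grid coordinates and flat 1D array indices.
; 2D-to-1D uses row-major X + Y * Width, returning -1 when X falls outside the width; Y is not bounds-checked.
; 1D-to-2D derives X from Index modulo Height and Y from Index divided by Width, so it inverts the first function only when Width equals Height.
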(fn `1D Index to 2D Index`
  (params (Index :type Integer) (Width :type Integer) (Height :type Integer))
  (returns (X :type Integer) (Y :type Integer))
  (return (mod Index Height) (/ Index Width)))

(fn `2D Index to 1D Index`
  (params (X :type Integer) (Y :type Integer) (Width :type Integer))
  (returns (Index :type Integer))
  (if (`KismetMathLibrary.InRange_IntInt` X 0 Width true false)
    (return (+ (`local.X`) (* (`local.Y`) (`local.Width`))))
    (else
      (return -1))))