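; Worker character Blueprint for an AI-driven worker that has an assigned house and worksite.
; On BeginPlay it calls SetupAssignments and prints the result with the house and worksite names as on-screen debug text.
; When possessed by an AIController, it runs its Behavior tree on that controller.
; The construction script and UpdateText function are empty.
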(event `self.ReceiveBeginPlay`
  (bind _returnvalue (`self.SetupAssignments`))
  (`KismetSystemLibrary.PrintText` (`|FormatText` "IsValid: {Valid} \nHouse: {House} \nWork: {Work}" _returnvalue (`KismetSystemLibrary.GetDisplayName` (`self.GetAssignedHouse`)) (`KismetSystemLibrary.GetDisplayName` (`self.GetAssignedWorksite`))) true false))

(event `self.ReceivePossessed`
  (params (NewController :type "Controller Object Reference"))
  (bind _asaicontroller (cast `AIController` NewController))
  (`AIController.RunBehaviorTree` _asaicontroller (`self.Behavior`)))

(fn `UpdateText`
  (locals (StringBuilder :type String)))

(fn `UserConstructionScript`)